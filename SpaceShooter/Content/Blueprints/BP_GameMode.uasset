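; Game mode for a space shooter that tracks progress, enemy kills and level, and handles the player's death.
; Progress rises by one about every second on Tick and by the score passed in on enemy deaths.
; Every second destroyed enemy raises the level.
; On player death it deactivates the BP_RandomGenerator found at BeginPlay, notifies BP_SpaceHUD and destroys all BP_EnemyBase actors.
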(event Custom|PlayerIsDead
  (Variables|/Game/Enemies/BP_RandomGenerator.BP_RandomGenerator_C|Setactivated (Variables|Default|GetenemyGenerator) false)
  (bind _asbp_space_hud (Utilities|Casting|CastToBP_SpaceHUD (HUD|GetHUD (Game|GetPlayerController 0))))
  (Default|PlayerIsDead _asbp_space_hud)
  (bind _outactors (Actor|GetAllActorsOfClass "/Game/Enemies/BP_EnemyBase.BP_EnemyBase_C"))
  (for _array_element _outactors
    (Actor|DestroyActor _array_element)))

(event Custom|EnemyDestroyed
  (bind _output_get (Variables|Default|SetEnemiesDestroyed (+ (Variables|Default|GetEnemiesDestroyed) 1)))
  (if (== (Math|Integer|%(Integer) _output_get 2) 0)
    (Variables|Default|SetLevel (+ (Variables|Default|GetLevel) 1))))

(event Custom|ScoreByEnemyDeath
  (params (newScore :type Integer))
  (Variables|Default|SetProgress (+ newScore (Variables|Default|GetProgress))))

(event EventBeginPlay
  (bind _returnvalue (Actor|GetActorOfClass "/Game/Enemies/BP_RandomGenerator.BP_RandomGenerator_C"))
  (Variables|Default|SetenemyGenerator _returnvalue))

(event EventTick
  (params (DeltaSeconds :type Float%20%28single-precision%29))
  (bind _output_get (Variables|Default|SetcountSeconds (+ DeltaSeconds (Variables|Default|GetcountSeconds))))
  (if (>= _output_get 1.0)
    (Variables|Default|SetProgress (+ (Variables|Default|GetProgress) 1))
    (Variables|Default|SetcountSeconds 0.0)))

(fn ConstructionScript)