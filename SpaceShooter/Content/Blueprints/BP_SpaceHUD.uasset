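; BP_SpaceHUD is the space game's HUD, showing the player's lives and game progress.
; On BeginPlay it creates the game widget, registers itself on the player character and caches the character and game mode.
; Tick polls both and pushes their values into the widget.
; PlayerIsDead plays a falling sound and notifies the widget that the player was killed.
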(event Custom|PlayerIsDead
  (Audio|PlaySound2D "/Game/Interface_And_Item_Sounds/WAV/Cartoon_Falling_05.Cartoon_Falling_05" 1.0 1.0 0.0 0 0)
  (Default|PlayerKilled (Variables|Default|GetGameWidget)))

(event EventBeginPlay
  (bind _returnvalue (Game|GetPlayerController 0))
  (Utilities|IsValid _returnvalue
    (:Is%20Valid
      (bind _returnvalue_2 (UserInterface|CreateWidget "/Game/Blueprints/BP_Space_GameWidget.BP_Space_GameWidget_C" _returnvalue))
      (bind _output_get (Variables|Default|SetGameWidget _returnvalue_2))
      (UserInterface|Viewport|AddtoViewport _output_get 0)
      ;[0.2719 0.2269 0.03673] CONECTAR CON JUGADOR
      (bind _asbp_space_character (Utilities|Casting|CastToBP_SpaceCharacter (Game|GetPlayerCharacter 0)))
      (Variables|Default|SetM_PlayerCharacter _asbp_space_character)
      (Variables|/Game/Players/BP_SpaceCharacter.BP_SpaceCharacter_C|SetHUD _asbp_space_character self)
      (bind _asbp_game_mode (Utilities|Casting|CastToBP_GameMode (Game|GetGameMode)))
      (Variables|Default|SetM_GameMode _asbp_game_mode))))

(event Collision|EventActorBeginOverlap
  (params (OtherActor :type Actor%20Object%20Reference)))

(event EventTick
  (params (DeltaSeconds :type Float%20%28single-precision%29))
  (bind _m_playercharacter (Variables|Default|GetM_PlayerCharacter))
  (Utilities|IsValid _m_playercharacter
    (:Is%20Valid
      (Default|UpdateWidgetValues (Variables|Default|GetGameWidget) (Variables|/Game/Players/BP_SpaceCharacter.BP_SpaceCharacter_C|GetLifes _m_playercharacter) (Variables|/Game/Blueprints/BP_GameMode.BP_GameMode_C|GetProgress (Variables|Default|GetM_GameMode))))))

(fn ConstructionScript)