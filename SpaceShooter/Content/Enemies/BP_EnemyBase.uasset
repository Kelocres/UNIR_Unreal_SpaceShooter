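; Base enemy actor that flies in a straight line, fires at a regular interval and awards score when killed.
; Tick moves it without sweep along the forward vector captured at BeginPlay and runs a timer that spawns Ammo at FirePoint.
; Any damage is lethal: it spawns an explosion, reports ScoreByDeath to BP_GameMode, then destroys the actor.
; The delayed Destroyed_Event handler is never bound, as its binding node is unconnected.
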(event Custom|Destroyed_Event
  (Utilities|FlowControl|Delay 0.2)
  (Actor|DestroyActor))

(event Custom|TakeDamageEvent
  (params (DamagedActor :type Actor%20Object%20Reference) (Damage :type Float%20%28single-precision%29) (DamageType :type Damage%20Type%20Object%20Reference) (InstigatedBy :type Controller%20Object%20Reference) (DamageCauser :type Actor%20Object%20Reference))
  (Effects|SpawnEmitteratLocation (Variables|Default|GetexplosionAtDeath) (Transformation|GetActorLocation))
  (bind _asbp_game_mode (Utilities|Casting|CastToBP_GameMode (Game|GetGameMode)))
  (Default|ScorebyEnemyDeath _asbp_game_mode (Variables|Default|GetscoreByDeath))
  (Actor|DestroyActor))

(event EventBeginPlay
  (Variables|Default|SetMovementVector (Transformation|GetActorForwardVector))
  (EventDispatchers|BindEventtoOnTakeAnyDamage (delegate Custom|TakeDamageEvent)))

(event Collision|EventActorBeginOverlap
  (params (OtherActor :type Actor%20Object%20Reference)))

(event EventTick
  (params (DeltaSeconds :type Float%20%28single-precision%29))
  (CallFunction|Move DeltaSeconds)
  (bind _output_get (Variables|Default|SetShotCurrentTime (+ (Variables|Default|GetShotCurrentTime) DeltaSeconds)))
  (if (> _output_get (Variables|Default|GetDelayShoot))
    (Variables|Default|SetShotCurrentTime 0.0)
    (CallFunction|Shoot)))

(fn ConstructionScript)

(fn Move
  (params (DeltaTime :type Float%20%28double-precision%29))
  (Transformation|SetActorLocation (+ (Transformation|GetActorLocation) (* (* DeltaTime (Variables|Default|GetSpeed)) (Variables|Default|GetMovementVector))) false false))

(fn Shoot
  (bind _returnvalue (Game|SpawnActorfromClass (Variables|Default|GetAmmo) (Transformation|GetWorldTransform (Variables|Default|GetFirePoint)) "Undefined" "MultiplyWithRoot" 0 0)))