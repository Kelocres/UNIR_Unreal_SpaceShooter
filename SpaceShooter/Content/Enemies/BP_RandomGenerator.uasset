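; BP_RandomGenerator is an enemy spawner that, while Activated, creates an enemy on a looping timer started at BeginPlay.
; Each spawn picks BP_EnemyBase or BP_EnemyH by a clamped random roll bounded by the game mode's Level.
; Location and rotation come from separate random picks among components tagged SpawnPoint.
; Each enemy's destroy event decrements SpawnTime, but the running timer is never reset with the new value.
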(event Custom|Spawn
  (if (Variables|Default|Getactivated)
    (bind _enemyspawned (CallFunction|SpawnEnemy))
    (bind _asbp_enemy_base (Utilities|Casting|CastToBP_EnemyBase _enemyspawned))
    (EventDispatchers|BindEventtoOnEnemyDestroy _asbp_enemy_base (delegate Custom|EnemyDestroyed))))

(event Custom|EnemyDestroyed
  (Variables|Default|SetSpawnTime (- (Variables|Default|GetSpawnTime) 1.0)))

(event EventBeginPlay
  (Variables|Default|Setactivated true)
  (Utilities|Time|SetTimerbyEvent (delegate Custom|Spawn) (Variables|Default|GetSpawnTime) true)
  (bind _asbp_game_mode (Utilities|Casting|CastToBP_GameMode (Game|GetGameMode)))
  (Variables|Default|Setm_GameMode _asbp_game_mode))

(fn ConstructionScript)

(fn SpawnEnemy
  (bind _returnvalue (Actor|GetComponentsbyTag "/Script/Engine.SceneComponent" "SpawnPoint"))
  (bind _returnvalue_2 (Utilities|Array|Length _returnvalue))
  (bind _returnvalue_3 (Math|Random|RandomInteger _returnvalue_2))
  (bind _output (Utilities|Array|Get(acopy) _returnvalue _returnvalue_3))
  (bind _returnvalue_4 (Transformation|GetWorldTransform _output))
  (bind _class (CallFunction|GetClasstoSpawn (Math|Random|RandomInteger (Variables|/Game/Blueprints/BP_GameMode.BP_GameMode_C|GetLevel (Variables|Default|Getm_GameMode)))))
  (bind _returnvalue_5 (Game|SpawnActorfromClass _class (Math|Transform|MakeTransform (.location _returnvalue_4) (.rotation _returnvalue_4) "1.000000,1.000000,1.000000") "AdjustIfPossibleButAlwaysSpawn" "MultiplyWithRoot" 0 0))
  (bind _asbp_enemy_base (Utilities|Casting|CastToBP_EnemyBase _returnvalue_5))
  (return _asbp_enemy_base))

(fn GetClasstoSpawn
  (params (Type :type Integer))
  (return (Utilities|Select :Index (Math|Integer|Clamp(Integer) Type 0 (- (Variables|Default|GetMaxNumEnemies) 0)) :Option%200 "/Game/Enemies/BP_EnemyBase.BP_EnemyBase_C" :Option%201 "/Game/Enemies/BP_EnemyH.BP_EnemyH_C")))