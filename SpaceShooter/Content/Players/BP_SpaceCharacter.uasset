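; Player-controlled space character that moves, shoots and loses lives when hit.
; BeginPlay adds an Enhanced Input mapping context and binds damage events, with input moving it along its right and forward vectors.
; Firing spawns ammo with a sound at the fire point, gated by a timer-reset cooldown.
; Any damage costs one life regardless of amount; at zero it notifies BP_GameMode, spawns an explosion and destroys itself.
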(event Custom|UpdateFire
  (Variables|Default|SetCanFire true))

(event Custom|OnTakeAnyDamage_Event
  (params (DamagedActor :type Actor%20Object%20Reference) (Damage :type Float%20%28single-precision%29) (DamageType :type Damage%20Type%20Object%20Reference) (InstigatedBy :type Controller%20Object%20Reference) (DamageCauser :type Actor%20Object%20Reference))
  (CallFunction|TakeDamage))

(event Input|EnhancedActionEvents|EnhancedInputActionBP_InputMovement
  (params (ActionValue :type Vector%202D%20Structure) (ElapsedSeconds :type Float%20%28double-precision%29) (TriggeredSeconds :type Float%20%28double-precision%29) (InputAction :type Input%20Action%20Object%20Reference :default "/Game/Blueprints/BP_InputMovement.BP_InputMovement"))
  ;[0.03558 0.1147 0.5927] MOVIMIENTO
  (Pawn|Input|AddMovementInput (Transformation|GetActorRightVector) (.x ActionValue) false)
  (Pawn|Input|AddMovementInput (Transformation|GetActorForwardVector) (.y ActionValue) false))

(event Input|EnhancedActionEvents|EnhancedInputActionBP_InputFire
  (params (ActionValue :type Boolean) (ElapsedSeconds :type Float%20%28double-precision%29) (TriggeredSeconds :type Float%20%28double-precision%29) (InputAction :type Input%20Action%20Object%20Reference :default "/Game/Blueprints/BP_InputFire.BP_InputFire"))
  (if (Variables|Default|GetCanFire)
    (CallFunction|DoFire)
    (Variables|Default|SetCanFire false)
    (Utilities|Time|SetTimerbyEvent (delegate Custom|UpdateFire) (Variables|Default|GetFireDelay))))

(event EventBeginPlay
  ;[0.1022 0.07713 0.4177] IMPLEMENTAR CONTROLES
  (bind _asplayer_controller (Utilities|Casting|CastToPlayerController (Pawn|GetController)))
  (Utilities|IsValid (PlayerController|LocalPlayerSubsystems|GetEnhancedInputLocalPlayerSubsystem _asplayer_controller)
    (:Is%20Valid
      (Input|AddMappingContext (PlayerController|LocalPlayerSubsystems|GetEnhancedInputLocalPlayerSubsystem _asplayer_controller) "/Game/Blueprints/BP_InputMapping.BP_InputMapping" 0 "(bIgnoreAllPressedKeysUntilRelease=True,bForceImmediately=False,bNotifyUserSettings=False)")
      (EventDispatchers|BindEventtoOnTakeAnyDamage (delegate Custom|OnTakeAnyDamage_Event)))
    (:Is%20Not%20Valid
      (Development|PrintText "PLAYER CONTROLLER IS NOT VALID"))))

(event Collision|EventActorBeginOverlap
  (params (OtherActor :type Actor%20Object%20Reference)))

(event EventTick
  (params (DeltaSeconds :type Float%20%28single-precision%29)))

(fn ConstructionScript)

(fn DoFire
  (bind _firepoint (Variables|Default|GetFirePoint))
  (bind _returnvalue (Transformation|GetWorldTransform _firepoint))
  (Game|SpawnActorfromClass (Variables|Default|GetAmmo) (Math|Transform|MakeTransform (.location _returnvalue) (.rotation _returnvalue) "1.000000,1.000000,1.000000") "Undefined" "MultiplyWithRoot" 0 0)
  (Audio|PlaySoundatLocation (Variables|Default|GetsoundAtShooting) (.location _returnvalue) "0, 0, 0" 1.0 1.0 0.0 0 0 0 0))

(fn TakeDamage
  (bind _returnvalue (Transformation|GetActorLocation))
  (bind _output_get (Variables|Default|SetLifes (- (Variables|Default|GetLifes) 1)))
  (if (== _output_get 0)
    (bind _asbp_game_mode (Utilities|Casting|CastToBP_GameMode (Game|GetGameMode)))
    (Default|PlayerIsDead _asbp_game_mode)
    (Effects|SpawnEmitteratLocation (Variables|Default|GetexplosionAtDeath) _returnvalue)
    (Actor|DestroyActor)
    (else
      (Audio|PlaySoundatLocation (Variables|Default|GetsoundAtDamage) _returnvalue "0, 0, 0" 1.0 1.0 0.0 0 0 0 0))))